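; A thrown VR disc projectile that returns to the player's right controller and breaks HexWall pieces it hits.
; EnableMovement switches it from physics to projectile movement and shows its trail.
; Tick enables homing once horizontal velocity exceeds 90 degrees from the player-to-enemy direction, destroys the disc near the controller, and prints debug network authority.
; On authority, hits destroy the struck wall component and spawn an impact effect.
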(event Custom|Enable%20Movement
  (params (Local%20Velocity :type Vector))
  (bind _projectilemovement (Variables|Default|GetProjectileMovement))
  (Game|Components|ProjectileMovement|SetVelocityinLocalSpace _projectilemovement Local%20Velocity)
  (Physics|SetSimulatePhysics (Variables|Default|GetDisc) false)
  (Components|Activation|Activate _projectilemovement false)
  (Rendering|SetVisibility (Variables|Default|GetTrail) true false))

(event Custom|Enable%20Homing
  (params (Homing%20Target :type Scene%20Component%20Object%20Reference))
  (bind _projectilemovement (Variables|Default|GetProjectileMovement))
  (Variables|/Script/Engine.ProjectileMovementComponent|SetHomingTargetComponent _projectilemovement Homing%20Target)
  (Variables|/Script/Engine.ProjectileMovementComponent|SetbIsHomingProjectile _projectilemovement true))

(event EventBeginPlay)

(event EventTick
  (params (DeltaSeconds :type Float%20%28single-precision%29))
  (Utilities|FlowControl|Sequence
    (:then_0
      (if (Components|Activation|IsActive (Variables|Default|GetProjectileMovement))
        (Utilities|IsValid (Variables|Default|GetVR_Character)
          (:Is%20Valid
            (Utilities|FlowControl|Sequence
              (:then_0
                ;[1 1 1] Enable Homing when Disc is returning
                (if (> (Class|KismetMathLibrary|DegAcos (Math|Vector|DotProduct (Variables|Default|GetDirectionFromPlayerToEnemy) (Math|Vector|Normalize (* (Transformation|GetVelocity) "1.000000,1.000000, 0")))) 9e+01)
                  (Utilities|FlowControl|DoOnce true :!label _label
                    (:Completed
                      (CallFunction|EnableHoming (Variables|/Game/Blueprints/VR_Character.VR_Character_C|Getvr_controller_R (Variables|Default|GetVR_Character)))))
                  (else
                    (goto _label Reset))))
              (:then_1
                ;[1 1 1] Destroy Disc when returned
                (if (and (Variables|/Script/Engine.ProjectileMovementComponent|GetbIsHomingProjectile (Variables|Default|GetProjectileMovement)) (< (Math|Vector|VectorLength (- (Transformation|GetActorLocation) (Transformation|GetWorldLocation (Variables|/Game/Blueprints/VR_Character.VR_Character_C|Getvr_controller_R (Variables|Default|GetVR_Character))))) 1e+02))
                  (Actor|DestroyActor))))))))
    (:then_1
      (Networking|SwitchHasAuthority
        (:Authority
          (Development|PrintString "Authority"))
        (:Remote
          (Development|PrintString "Remote" true true "(R=0.000000,G=1.000000,B=0.833333,A=1.000000)"))))))

(event Collision|EventHit
  (params (MyComp :type Primitive%20Component%20Object%20Reference) (Other :type Actor%20Object%20Reference) (OtherComp :type Primitive%20Component%20Object%20Reference) (bSelfMoved :type Boolean) (HitLocation :type Vector) (HitNormal :type Vector :default "0, 0, 0") (NormalImpulse :type Vector :default "0, 0, 0") (Hit :type Hit%20Result%20Structure%20%28by%20ref%29))
  (Networking|SwitchHasAuthority
    (:Authority
      (Utilities|Casting|CastToHexWall Other)
      (Components|DestroyComponent OtherComp)
      (Effects|SpawnEmitteratLocation "/Game/Particles/Tor_Treffer.Tor_Treffer" HitLocation (Math|Rotator|FindLookatRotation (* HitLocation "1.000000,1.000000, 0") (Math|Vector|MakeVector 0.0 0.0 0.0))))))

(fn ConstructionScript)