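; Server-authoritative spawner that keeps launching a Disc actor from its own transform, replacing it once the previous one is gone.
; Tick waits briefly when no valid disc exists, spawns one with the spawner's root as homing target, swaps its material and enables movement.
; Velocity comes from GetDirectionInCone in disc-local space, though that function's random-spread, speed-scaled forward calculation appears unconnected.
; Each disc is destroyed after Lifetime.
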(event EventBeginPlay)

(event Collision|EventActorBeginOverlap
  (params (OtherActor :type Actor%20Object%20Reference)))

(event EventTick
  (params (DeltaSeconds :type Float%20%28single-precision%29))
  (Networking|SwitchHasAuthority
    (:Authority
      (Utilities|IsValid (Variables|Default|GetSpawnedDisc)
        (:Is%20Not%20Valid
          (Utilities|FlowControl|Delay 0.5)
          (bind _returnvalue (Game|SpawnActorfromClass "/Game/Blueprints/Disc.Disc_C" (Transformation|GetActorTransform) "Undefined" 0 0 (Variables|Default|GetDefaultSceneRoot)))
          (bind _output_get (Variables|Default|SetSpawnedDisc _returnvalue))
          (Rendering|Material|SetMaterial (Variables|/Game/Blueprints/Disc.Disc_C|GetDisc _output_get) 1 "/Game/Materials/BaseMat_Inst2.BaseMat_Inst2")
          (Default|EnableMovement _output_get (Math|Transform|InverseTransformDirection (Transformation|GetActorTransform _output_get) (|GetDirectionInCone)))
          (Utilities|FlowControl|Delay (Variables|Default|GetLifetime))
          (Actor|DestroyActor (Variables|Default|GetSpawnedDisc)))))))

(fn ConstructionScript)