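; Game mode for a two-player VR match that runs a countdown, decides the winner and restarts the level.
; PostLogin tags each player's VR_Character by join order and teleports the second to the first MyPlayerStart.
; Tick updates the clamped timer and checks for a player's hex wall count reaching zero, or compares scores at timeout.
; The result prints on screen, and the current level reopens after a short delay.
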(event EventTick
  (params (DeltaSeconds :type Float%20%28single-precision%29))
  (Utilities|FlowControl|Sequence
    (:then_0
      (CallFunction|UpdateTimer)
      (Utilities|CheckWinConditions
        (:P1%20Wins
          (Development|PrintString "WIN P1" true true "(R=1.000000,G=1.000000,B=1.000000,A=1.000000)" 5.0))
        (:Draw
          (Development|PrintString "DRAW" true true "(R=1.000000,G=1.000000,B=0.000000,A=1.000000)" 5.0))
        (:P2%20Wins
          (Development|PrintString "WIN P2" true true "(R=1.000000,G=0.000000,B=0.000000,A=1.000000)" 5.0)))
      (Utilities|FlowControl|Delay 5.0)
      (bind _returnvalue (Game|GetCurrentLevelName true))
      (Game|OpenLevel(byName) (Utilities|String|StringToName _returnvalue)))))

(event EventBeginPlay
  (CallFunction|InitGame))

(event EventPostLogin
  (params (NewPlayer :type Player%20Controller%20Object%20Reference))
  (bind _returnvalue (Pawn|GetControlledPawn NewPlayer))
  (bind _returnvalue_2 (Class|GameMode|GetNumPlayers))
  (switch int _returnvalue_2
    (:1
      (bind _asvr_character (Utilities|Casting|CastToVR_Character _returnvalue))
      (Variables|/Game/Blueprints/VR_Character.VR_Character_C|SetPlayerTag _asvr_character "NewEnumerator0"))
    (:2
      (bind _asvr_character_2 (Utilities|Casting|CastToVR_Character _returnvalue))
      (Variables|/Game/Blueprints/VR_Character.VR_Character_C|SetPlayerTag _asvr_character_2 "NewEnumerator1")
      (bind _outactors (Actor|GetAllActorsOfClass "/Game/Blueprints/MyPlayerStart.MyPlayerStart_C"))
      (Transformation|Teleport (Pawn|GetControlledPawn NewPlayer) (.location (Transformation|GetActorTransform (Utilities|Array|Get(acopy) _outactors))) (.rotation (Transformation|GetActorTransform (Utilities|Array|Get(acopy) _outactors)))))))

(fn ConstructionScript)

(fn InitGame
  (Variables|Default|SetTime (Variables|Default|GetMaxTime)))

(fn UpdateTimer
  (Variables|Default|SetTime (Math|Float|Clamp(Float) (- (Variables|Default|GetTime) (Utilities|Time|GetWorldDeltaSeconds)) 0.0 (Variables|Default|GetMaxTime)))
  (return))