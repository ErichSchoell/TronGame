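; VR player character that holds a Disc at a right-hand physics handle and lets the player throw it.
; Tick moves the handle to DiscSpawnPoint and spawns a new disc, grabbed by the handle, whenever no valid one exists.
; Releasing the right trigger drops the grab and passes the disc's velocity, converted to local space and doubled, to its EnableMovement.
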(event Custom|Spawn%20Disc
  (bind _discspawnpoint (Variables|Default|GetDiscSpawnPoint))
  (bind _returnvalue (Game|SpawnActorfromClass "/Game/Blueprints/Disc.Disc_C" (Math|Transform|MakeTransform (+ (Transformation|GetWorldLocation _discspawnpoint) (* (Math|Vector|GetForwardVector _discspawnpoint) 1e+01)) (Transformation|GetWorldRotation _discspawnpoint) "1.500000,1.500000,1.500000") "AlwaysSpawn" 0 0))
  (bind _output_get (Variables|Default|SetSpawnedDisc _returnvalue))
  (Variables|/Game/Blueprints/Disc.Disc_C|SetVR_Character _output_get self)
  (Class|PhysicsHandleComponent|GrabComponent (Variables|Default|GetPhysicsHandleR) (Variables|/Game/Blueprints/Disc.Disc_C|GetDisc (Variables|Default|GetSpawnedDisc)) "None" (Transformation|GetActorLocation (Variables|Default|GetSpawnedDisc)) true))

(event EventTick
  (params (DeltaSeconds :type Float%20%28single-precision%29))
  (bind _discspawnpoint (Variables|Default|GetDiscSpawnPoint))
  (Class|PhysicsHandleComponent|SetTargetLocationandRotation (Variables|Default|GetPhysicsHandleR) (Transformation|GetWorldLocation _discspawnpoint) (Transformation|GetWorldRotation _discspawnpoint))
  (Utilities|IsValid (Variables|Default|GetSpawnedDisc)
    (:Is%20Not%20Valid
      (CallFunction|SpawnDisc))))

(event EventBeginPlay)

(event Input|KeyboardEvents|MotionControllerRightTrigger
  (params (Key :type Key%20Structure :default "AnyKey"))
  (bind _spawneddisc (Variables|Default|GetSpawnedDisc))
  (:Released
    (Utilities|IsValid _spawneddisc
      (:Is%20Valid
        (Physics|Components|PhysicsHandle|ReleaseComponent (Variables|Default|GetPhysicsHandleR))
        (Default|EnableMovement _spawneddisc (* (Math|Transform|InverseTransformDirection (Transformation|GetActorTransform _spawneddisc) (Transformation|GetVelocity _spawneddisc)) 2.0))))))

(event Input|KeyboardEvents|MotionControllerLeftTrigger
  (params (Key :type Key%20Structure :default "AnyKey")))

(fn ConstructionScript)