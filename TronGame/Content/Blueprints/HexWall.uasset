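; HexWall is a destructible wall Blueprint built from static mesh pieces that a Disc breaks apart on contact.
; When a Disc hits it, the struck component is destroyed and a particle effect spawns at the hit location.
; Tick counts the remaining static mesh components, and once none are left it waits briefly, then reloads the current level.
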(event EventBeginPlay)

(event EventTick
  (params (DeltaSeconds :type Float%20%28single-precision%29))
  (if (== (Utilities|Array|Length (Actor|GetComponentsByClass "/Script/Engine.StaticMeshComponent")) 0)
    (Utilities|FlowControl|Delay 1.5)
    (bind _returnvalue (Game|GetCurrentLevelName true))
    (Game|OpenLevel(byName) (Utilities|String|StringToName _returnvalue))))

(event Collision|EventHit
  (params (MyComp :type Primitive%20Component%20Object%20Reference) (Other :type Actor%20Object%20Reference) (OtherComp :type Primitive%20Component%20Object%20Reference) (bSelfMoved :type Boolean) (HitLocation :type Vector) (HitNormal :type Vector :default "0, 0, 0") (NormalImpulse :type Vector :default "0, 0, 0") (Hit :type Hit%20Result%20Structure%20%28by%20ref%29))
  (Utilities|Casting|CastToDisc Other)
  (Components|DestroyComponent MyComp)
  (Effects|SpawnEmitteratLocation "/Game/Particles/TestParticle.TestParticle" HitLocation))

(fn ConstructionScript)