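; TestAngle is a test actor that visualizes a ricocheting line trace from the player pawn toward its own location every tick.
; Ricochet traces on the Visibility channel, then mirrors the incoming direction about the impact normal to cast a fixed-length follow-up trace.
; It loops by feeding each hit back in until a trace misses or the bounce limit is exceeded, drawing debug lines for one frame.
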(event EventBeginPlay)

(event Collision|EventActorBeginOverlap
  (params (OtherActor :type Actor%20Object%20Reference)))

(event EventTick
  (params (DeltaSeconds :type Float%20%28single-precision%29))
  (CallFunction|Ricochet (Transformation|GetActorLocation (Game|Player|GetPlayerPawn 0)) (Transformation|GetActorLocation) 2))

(fn ConstructionScript)

(fn Ricochet
  (params (From :type Vector) (To :type Vector) (MaxBounces :type Integer))
  (Utilities|FlowControl|Sequence
    (:then_0
      (LocalVariables|SetStartPoint From)
      (LocalVariables|SetEndPoint To)
      (LocalVariables|Set_MaxBounces MaxBounces))
    (:then_1
      (bind _outhit (Collision|LineTraceByChannel (LocalVariables|GetStartPoint) (LocalVariables|GetEndPoint) "TraceTypeQuery1" false 0 "ForOneFrame" false))
      (LocalVariables|SetImpactPoint (.ImpactPoint (Collision|BreakHitResult _outhit)))
      (LocalVariables|SetImpactNormal (.ImpactNormal (Collision|BreakHitResult _outhit)))
      (bind (_outhit_2 _returnvalue) (Collision|LineTraceByChannel (LocalVariables|GetImpactPoint) (+ (LocalVariables|GetImpactPoint) (Math|Vector|MirrorVectorbyNormal (* (Class|KismetMathLibrary|GetDirectionVector (LocalVariables|GetStartPoint) (LocalVariables|GetEndPoint)) 2e+03) (LocalVariables|GetImpactNormal))) "TraceTypeQuery1" false 0 "ForOneFrame" :!label _label))
      (bind _result (Math|Integer|IncrementInt (LocalVariables|GetBounceCount))
        (:%20%20
          (if (and _returnvalue (<= _result (LocalVariables|Get_MaxBounces)))
            (Utilities|FlowControl|Sequence
              (:then_0
                (LocalVariables|SetImpactPoint (.ImpactPoint (Collision|BreakHitResult _outhit_2))))
              (:then_1
                (LocalVariables|SetImpactNormal (.ImpactNormal (Collision|BreakHitResult _outhit_2))))
              (:then_2
                (LocalVariables|SetStartPoint (.TraceStart (Collision|BreakHitResult _outhit_2))))
              (:then_3
                (LocalVariables|SetEndPoint (.TraceEnd (Collision|BreakHitResult _outhit_2))))
              (:then_4
                (goto _label)))
            (else
              (return))))))))